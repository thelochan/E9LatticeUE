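; Planet actor that orbits a center point, following CenterActor's location when one is valid, at a configurable Speed.
; Each Tick it re-orthogonalizes the orbit Axis against the radius using cross products, rotates its offset around that axis, and prints the orbit radius for debugging.
; The construction script applies the texture and intensity through a dynamic material and sets RotatingMovement's spin rate.
; Debug line drawing for radius and axis is left disconnected.
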(event Custom|OrthogonalizeAxis
  (bind _returnvalue (Transformation|GetActorLocation))
  (bind _centerlocation (Variables|Default|GetCenterLocation))
  (bind _returnvalue_2 (- _returnvalue _centerlocation))
  (Variables|Default|SetAxis (Math|Vector|Normalize (Math|Vector|CrossProduct _returnvalue_2 (Math|Vector|CrossProduct (Variables|Default|GetAxis) _returnvalue_2)))))

(event EventTick
  (params (DeltaSeconds :type Float%20%28single-precision%29))
  (Utilities|FlowControl|Sequence
    (:then_0
      (bind _centeractor (Variables|Default|GetCenterActor)
        (:then
          (Variables|Default|SetCenterLocation (Transformation|GetActorLocation _centeractor)))
        (:else)))
    (:then_1
      (CallFunction|OrthogonalizeAxis)
      (Transformation|SetActorLocation (+ (Math|Vector|RotateVectorAroundAxis (- (Transformation|GetActorLocation) (Variables|Default|GetCenterLocation)) (* DeltaSeconds (Variables|Default|GetSpeed)) (Variables|Default|GetAxis)) (Variables|Default|GetCenterLocation)) false false)
      (Development|PrintString (Utilities|String|ToString(Float) (Math|Vector|VectorLength (- (Transformation|GetActorLocation) (Variables|Default|GetCenterLocation)))) true true "(R=0.000000,G=0.660000,B=1.000000,A=1.000000)" 0.0))))

(fn ConstructionScript
  (bind _returnvalue (Rendering|Material|CreateDynamicMaterialInstance (Variables|Default|GetSphere) 0 "/Game/Textures/Planet_Mat.Planet_Mat" "None" :!class /Script/Engine.PrimitiveComponent))
  (Rendering|Material|SetTextureParameterValue _returnvalue "PlanetTexture" (Variables|Material|GetPlanetTexture))
  (Rendering|Material|SetScalarParameterValue _returnvalue "Intensity" (Variables|Material|GetIntensity) :!class /Script/Engine.MaterialInstanceDynamic)
  (Variables|/Script/Engine.RotatingMovementComponent|SetRotationRate (Variables|Default|GetRotatingMovement) (Variables|Default|GetRotation%20Rate)))